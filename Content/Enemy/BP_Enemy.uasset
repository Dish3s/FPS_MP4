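; BP_Enemy is a flipbook-sprite enemy that chases and hurts the first-person player.
; PawnSensing sets CanSeePlayer, which is never cleared, and starts AIMoveTo toward the player, while Tick yaws the actor to face them.
; Overlapping the player applies fixed damage.
; Incoming damage drains EnemyHealth; at zero, a DoOnce stops movement, plays a non-looping death flipbook, then destroys the actor after a delay.
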(event OnSeePawn(PawnSensing)
  (params (Pawn :type Pawn%20Object%20Reference))
  ;[0.01961 0.01961 0.01961] Sense the character
  (bind _asbp_first_person_character (Utilities|Casting|CastToBP_FirstPersonCharacter Pawn))
  (Variables|Default|SetcanSeePlayer true)
  (AI|AIMoveTo self "0, 0, 0" _asbp_first_person_character 5.0 false))

(event Collision|EventActorBeginOverlap
  (params (OtherActor :type Actor%20Object%20Reference))
  (bind _asbp_first_person_character (Utilities|Casting|CastToBP_FirstPersonCharacter OtherActor))
  (Game|Damage|ApplyDamage _asbp_first_person_character 2e+01 0 0))

(event EventTick
  (params (DeltaSeconds :type Float%20%28single-precision%29))
  ;[0.01562 0.01562 0.01562] Can see the player
  (if (Variables|Default|GetcanSeePlayer)
    (Transformation|SetActorRotation (Math|Rotator|MakeRotator 0.0 0.0 (.yaw (Math|Rotator|FindLookatRotation (Transformation|GetActorLocation) (Transformation|GetActorLocation (Game|GetPlayerCharacter 0))))))))

(event Game|Damage|EventAnyDamage
  (params (Damage :type Float%20%28single-precision%29) (DamageType :type Damage%20Type%20Object%20Reference) (InstigatedBy :type Controller%20Object%20Reference) (DamageCauser :type Actor%20Object%20Reference))
  (bind _output_get (Variables|Default|SetEnemyHealth (- (Variables|Default|GetEnemyHealth) Damage)))
  (if (<= _output_get 0.0)
    (Utilities|FlowControl|DoOnce false
      (:Completed
        (Components|Activation|Deactivate (Variables|Character|GetCharacterMovement))
        (Sprite|SetFlipbook (Variables|Default|GetPaperFlipbook) (Variables|Default|GetDeathAnime))
        (Components|Timeline|SetLooping (Variables|Default|GetPaperFlipbook) false)
        (Utilities|FlowControl|Delay 4.0)
        (Actor|DestroyActor)))))

(fn ConstructionScript)