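; Submachine gun weapon Blueprint that handles firing and its Paper2D flipbook animation.
; ShootWeapon passes through a DoOnce gate, calls FireWeapon and switches the weapon flipbook to the firing animation.
; After a delay equal to that flipbook's length, it restores the idle flipbook and calls ResetWeapon to reopen the gate, so fire rate follows animation length.
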(event Custom|ResetWeapon
  (bind _weaponflipbook (Variables|Default|GetWeaponflipbook))
  (Utilities|FlowControl|DoOnce false) ; enters at Reset
)

(event EventBeginPlay)

(event Collision|EventActorBeginOverlap
  (params (OtherActor :type Actor%20Object%20Reference)))

(event EventTick
  (params (DeltaSeconds :type Float%20%28single-precision%29)))

(event EventShootWeapon
  (bind _weaponflipbook (Variables|Default|GetWeaponflipbook))
  (Utilities|FlowControl|DoOnce false
    (:Completed
      (CallFunction|FireWeapon)
      (Sprite|SetFlipbook _weaponflipbook "/Game/Blueprint/Weapons/Submachinegun1.Submachinegun1")
      (Utilities|FlowControl|Delay (Class|PaperFlipbookComponent|GetFlipbookLength _weaponflipbook))
      (Sprite|SetFlipbook (Variables|Default|GetWeaponflipbook) "/Game/Blueprint/Weapons/Sub_Idle.Sub_Idle")
      (CallFunction|ResetWeapon self))))

(fn ConstructionScript
  (|CallParentFunction))